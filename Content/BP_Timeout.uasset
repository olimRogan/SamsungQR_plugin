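; BP_Timeout is an idle timer that opens the "Start" level when pointer input has not moved over a timeout interval.
; Each Tick runs either the Mouse or Touch check depending on IsTouchMode, adding delta time until ten times the elapsed time reaches OutTime.
; It then compares the current mouse or first-touch position with the stored one, returning to Start if identical, otherwise saving it and restarting the timer.
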(event EventBeginPlay
  (if (Variables|Default|GetIs%20Touch%20Mode)
    (bind _returnvalue (CallFunction|GetTouchPos))
    (Variables|Default|SetPreTouchPos _returnvalue)
    (else
      (bind _returnvalue_2 (Class|WidgetLayoutLibrary|GetMousePositiononViewport))
      (Variables|Default|SetPreMousePos _returnvalue_2))))

(event EventTick
  (params (DeltaSeconds :type Float%20%28single-precision%29))
  (if (Variables|Default|GetIs%20Touch%20Mode)
    (CallFunction|Touch DeltaSeconds)
    (else
      (CallFunction|Mouse DeltaSeconds))))

(fn ConstructionScript)

(fn Mouse
  (params (Delta :type Float%20%28single-precision%29))
  (bind _returnvalue (Class|WidgetLayoutLibrary|GetMousePositiononViewport))
  (Variables|Default|SetCurMousePos _returnvalue)
  (bind _output_get (Variables|Default|SetTime (+ (Variables|Default|GetTime) Delta)))
  (if (>= (* _output_get 1e+01) (Variables|Default|GetOutTime))
    (if (Class|KismetMathLibrary|EqualExactlyVector2DVector2D (Variables|Default|GetPreMousePos) (Variables|Default|GetCurMousePos))
      (Variables|Default|SetTime 0.0)
      (Game|OpenLevel(byName) "Start")
      (else
        (Utilities|FlowControl|DoOnce false :!label _label
          (:Completed
            (Variables|Default|SetPreMousePos (Variables|Default|GetCurMousePos))
            (Variables|Default|SetTime 0.0)
            (goto _label Reset)))))))

(fn GetTouchPos
  (bind _returnvalue (Game|GetPlayerController 0))
  (bind (_locationx _locationy) (Class|PlayerController|GetInputTouchState _returnvalue "Touch1"))
  (return (Math|Vector2D|MakeVector2D _locationx _locationy)))

(fn Touch
  (params (Delta :type Float%20%28single-precision%29))
  (bind _returnvalue (CallFunction|GetTouchPos))
  (Variables|Default|SetCurTouchPos _returnvalue)
  (bind _output_get (Variables|Default|SetTime (+ (Variables|Default|GetTime) Delta)))
  (if (>= (* _output_get 1e+01) (Variables|Default|GetOutTime))
    (if (Class|KismetMathLibrary|EqualExactlyVector2DVector2D (Variables|Default|GetPreTouchPos) (Variables|Default|GetCurTouchPos))
      (Variables|Default|SetTime 0.0)
      (Game|OpenLevel(byName) "Start")
      (else
        (Utilities|FlowControl|DoOnce false :!label _label
          (:Completed
            (Variables|Default|SetPreTouchPos (Variables|Default|GetCurTouchPos))
            (Variables|Default|SetTime 0.0)
            (goto _label Reset)))))))